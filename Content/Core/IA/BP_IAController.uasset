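; BP_IAController is an AI controller that moves a BP_IAClient pawn to action points and exits.
; Every Tick, without a valid target it picks a random BP_ActionPNJ, registers its client as that actor's IAToGet, and reissues a simple move toward it.
; When IsLeaving is set, it instead moves toward a random ExitPoint entry, re-rolled each frame.
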(event EventTick
  (params (DeltaSeconds :type Float%20%28single-precision%29))
  (if (Variables|Default|GetIsLeaving)
    (AI|Navigation|SimpleMovetoLocation self (.OutItem (Utilities|Array|Random (Variables|Default|GetExitPoint))))
    (else
      (if (Utilities|IsValid (Variables|Default|GetObjectifPos))
        _
        (else
          (bind _asbp_iaclient (Utilities|Casting|CastToBP_IAClient (Pawn|GetControlledPawn self)))
          (Variables|Default|SetAs%20BP%20IAClient _asbp_iaclient)
          (bind _outactors (Actor|GetAllActorsOfClass "/Game/Core/Environement/BP_ActionPNJ.BP_ActionPNJ_C"))
          (bind _output_get (Variables|Default|SetObjectifPos (.OutItem (Utilities|Array|Random _outactors))))
          (Variables|/Game/Core/Environement/BP_ActionPNJ.BP_ActionPNJ_C|SetIAToGet _output_get (Variables|Default|GetAs%20BP%20IAClient))))
      (AI|Navigation|SimpleMovetoActor self _output_get))))

(fn ConstructionScript)