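; BP_ActionPNJ is a table spot where an assigned NPC sits, orders food and eats.
; When that NPC enters DetectPlayer, the table marks it seated, registers itself as its ActualTable and triggers OrderFood.
; FoodServed flags the NPC as eating and spawns a new actor of the served food's class at SpawnFood2.
; FinishEat destroys that food and clears the NPC, awaited food and occupied flag.
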(event OnComponentBeginOverlap(DetectPlayer)
  (params (OverlappedComponent :type Primitive%20Component%20Object%20Reference) (OtherActor :type Actor%20Object%20Reference) (OtherComp :type Primitive%20Component%20Object%20Reference) (OtherBodyIndex :type Integer) (bFromSweep :type Boolean) (SweepResult :type Hit%20Result%20Structure%20%28by%20ref%29))
  (bind _iatoget (Variables|Default|GetIAToGet))
  (if (== OtherActor (Variables|Default|GetIAToGet))
    (Variables|/Game/Core/IA/BP_IAClient.BP_IAClient_C|SetIsSitting _iatoget true)
    (Variables|/Game/Core/IA/BP_IAClient.BP_IAClient_C|SetActualTable _iatoget self)
    (Default|OrderFood _iatoget)
    (Variables|Default|SetIaSitted true)))

(event OnComponentEndOverlap(DetectPlayer)
  (params (OverlappedComponent :type Primitive%20Component%20Object%20Reference) (OtherActor :type Actor%20Object%20Reference) (OtherComp :type Primitive%20Component%20Object%20Reference) (OtherBodyIndex :type Integer)))

(event Custom|FoodServed
  (params (GettedFood :type BP%20Food%20Parent%20Object%20Reference))
  (Variables|/Game/Core/IA/BP_IAClient.BP_IAClient_C|SetIsEating (Variables|Default|GetIAToGet) true)
  (bind _returnvalue (Game|SpawnActorfromClass (Utilities|GetClass GettedFood) (Transformation|GetWorldTransform (Variables|Default|GetSpawnFood2)) "AlwaysSpawn" "OverrideRootScale" 0 0))
  (Variables|Default|SetPlacedFoodRef _returnvalue))

(event Custom|FinishEat
  (Variables|Default|SetIAToGet 0)
  (Variables|Default|SetWaitedfood 0)
  (Actor|DestroyActor (Variables|Default|GetPlacedFoodRef))
  (Variables|Default|SetIaSitted false))

(fn ConstructionScript)