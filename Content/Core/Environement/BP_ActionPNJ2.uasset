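; BP_ActionPNJ2 is an environment action actor that cooks food for a player and puts it in their hands.
; CookFood stores the controller and its BP_Player pawn, sets IsCooking, then starts a short timer.
; The timer routes through server and multicast events, which spawn a BP_FoodParent inside the multicast.
; The food loses mesh collision, attaches to the player's HoldPoint and is recorded as held.
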(event Custom|CookFood
  (params (ControllerRef :type BP%20Player%20Controller%20Object%20Reference))
  (bind _output_get (Variables|Default|SetAs%20BP%20Controller ControllerRef))
  (bind _asbp_player (Utilities|Casting|CastToBP_Player (Pawn|GetControlledPawn _output_get)))
  (bind _output_get_2 (Variables|Default|SetAs%20BP%20Player _asbp_player))
  (Variables|/Game/Core/BP_Player.BP_Player_C|SetIsCooking _output_get_2 true)
  (Utilities|Time|SetTimerbyEvent (delegate Custom|SpawnFood) 2.0))

(event Custom|SpawnFood
  (CallFunction|ServerSpawnFood))

(event Custom|Server_SpawnFood
  (CallFunction|MultiCastSpawnFood))

(event Custom|MultiCast_SpawnFood
  (Variables|/Game/Core/BP_Player.BP_Player_C|SetIsCooking (Variables|Default|GetAs%20BP%20Player) false)
  (bind _returnvalue (Game|SpawnActorfromClass "/Game/Core/Items/BP_FoodParent.BP_FoodParent_C" (Transformation|GetActorTransform self) "Undefined" "MultiplyWithRoot" 0 0))
  (Collision|SetCollisionEnabled (Variables|/Game/Core/Items/BP_FoodParent.BP_FoodParent_C|GetStaticMesh _returnvalue) "NoCollision")
  (Transformation|AttachComponentToComponent _returnvalue (Variables|/Game/Core/BP_Player.BP_Player_C|GetHoldPoint (Variables|Default|GetAs%20BP%20Player)) "None" "SnapToTarget" "SnapToTarget" "KeepWorld" true)
  (Variables|/Game/Core/BP_Player.BP_Player_C|SetIsHolding (Variables|Default|GetAs%20BP%20Player) true)
  (Variables|/Game/Core/BP_PlayerController.BP_PlayerController_C|SetFoodHolding (Variables|Default|GetAs%20BP%20Controller) _returnvalue))

(fn ConstructionScript)