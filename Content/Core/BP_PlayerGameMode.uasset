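; Game mode that starts the match, spawns AI clients and tracks when all player controllers are ready.
; On BeginPlay, a looping timer spawns BP_IAClient at random spawn points, with its interval randomized once at setup; the HUD step is empty.
; Tick polls every BP_PlayerController for client readiness.
; While the ready count matches the expected total, it re-runs camera setup on each controller every frame.
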(event Custom|StartGame
  (CallFunction|SpawnHUD)
  (CallFunction|SpawnClients)
  (Variables|Default|SetGameStart true))

(event Custom|SpawnClients
  (Utilities|Time|SetTimerbyEvent (delegate Custom|SpawnClient) (Math|Random|RandomFloatinRange 8.0 15.0) true))

(event Custom|AllPlayersReady
  (for _array_element (Variables|Default|GetPlayerControllersReady)
    (Default|SetCamera _array_element)))

(event Custom|SpawnHUD)

(event Custom|SpawnClient
  (Game|SpawnActorfromClass "/Game/Core/IA/BP_IAClient.BP_IAClient_C" (Math|Conversions|ToTransform(Vector) (.OutItem (Utilities|Array|Random (Variables|Default|GetClientSpawnPoint)))) "AlwaysSpawn" "MultiplyWithRoot" 0 0))

(event EventBeginPlay
  (CallFunction|StartGame))

(event EventTick
  (params (DeltaSeconds :type Float%20%28single-precision%29))
  (if true
    (bind _outactors (Actor|GetAllActorsOfClass "/Game/Core/BP_PlayerController.BP_PlayerController_C"))
    (for _array_element _outactors
      (if (Variables|/Game/Core/BP_PlayerController.BP_PlayerController_C|GetIsClientReady _array_element)
        (if (not (Utilities|Array|ContainsItem (Variables|Default|GetPlayerControllersReady) _array_element))
          (Utilities|Array|Add (Variables|Default|GetPlayerControllersReady) _array_element))))
    (if (== (Utilities|Array|Length (Variables|Default|GetPlayerControllersReady)) (Variables|Default|GetTotalPlayerController))
      (Variables|Default|SetAllPlayerReady true)
      (CallFunction|AllPlayersReady))))

(fn ConstructionScript)